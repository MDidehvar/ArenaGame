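; Arena player controller that lets a player without a pawn request a respawn.
; Pressing P calls a server respawn request when no valid controlled pawn exists.
; The request event casts the game mode to Arena_GameMode and passes this controller to its ServerRespawnPlayer, leaving the respawn itself to the game mode.
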(event Custom|Server_RequestRespawn
  (bind _returnvalue (Game|GetGameMode))
  (Utilities|IsValid _returnvalue
    (:Is%20Valid
      (bind _asarena_game_mode (Utilities|Casting|CastToArena_GameMode _returnvalue))
      (Utilities|IsValid _asarena_game_mode
        (:Is%20Valid
          (Default|ServerRespawnPlayer _asarena_game_mode self))))))

(event Input|KeyboardEvents|P
  (params (Key :type Key%20Structure))
  ;[1 1 1] Request to Respawn Player
  (:Pressed
    (Utilities|IsValid (Pawn|GetControlledPawn self)
      (:Is%20Not%20Valid
        (CallFunction|ServerRequestRespawn)))))

(fn ConstructionScript)