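; Arena game mode that respawns players as a new Archer_Character.
; BeginPlay caches every PlayerStart in SpawnPoints.
; Server_RespawnPlayer spawns the archer at GetRandomSpawnPoint's transform, ignoring collisions, and has the given controller possess it.
; GetRandomSpawnPoint contains random-pick logic over SpawnPoints, but it is left unused, with no visible output connection.
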(event Custom|Server_RespawnPlayer
  (params (PlayerController :type Player%20Controller%20Object%20Reference))
  (bind (_returnvalue_location _returnvalue_rotation) (Utilities|GetRandomSpawnPoint))
  (Utilities|IsValid PlayerController
    (:Is%20Valid
      (bind _returnvalue (Game|SpawnActorfromClass "/Game/Blueprints/Archer_Character.Archer_Character_C" (Math|Transform|MakeTransform _returnvalue_location _returnvalue_rotation "1,1,1") "AlwaysSpawn" 0 0))
      (Utilities|IsValid _returnvalue
        (:Is%20Valid
          (Pawn|Possess PlayerController _returnvalue))))))

(event EventBeginPlay
  (bind _outactors (Actor|GetAllActorsOfClass "/Script/Engine.PlayerStart"))
  (Variables|Default|SetSpawnPoints _outactors))

(fn ConstructionScript)