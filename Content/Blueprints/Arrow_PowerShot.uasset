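; Power-shot arrow projectile that damages whatever it hits, crediting the instigator's controller.
; On hit it applies damage, calls MulticastEmitter for the impact particle, quiet sound and collision shutoff, then shortens its remaining life to a few seconds.
; A delayed velocity-set workaround for client impact collision in multiplayer is left disconnected, so BeginPlay does nothing.
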(event Custom|MulticastEmitter
  (bind _returnvalue (Transformation|GetActorLocation))
  ;[0 0 0] Arrow Collision
  (Effects|SpawnEmitteratLocation (Variables|Default|GetHitEffect) _returnvalue)
  (Audio|PlaySoundatLocation "/Game/Extras/Sound/SniperRifle/Wavs/SniperRifle_ImpactSurface01.SniperRifle_ImpactSurface01" _returnvalue "0, 0, 0" 0.1 1.0 0.0 "/Game/Impact_Attenuation.Impact_Attenuation")
  (Collision|SetActorEnableCollision false))

(event Collision|EventHit
  (params (MyComp :type Primitive%20Component%20Object%20Reference) (Other :type Actor%20Object%20Reference) (OtherComp :type Primitive%20Component%20Object%20Reference) (bSelfMoved :type Boolean) (HitLocation :type Vector :default "0, 0, 0") (HitNormal :type Vector :default "0, 0, 0") (NormalImpulse :type Vector :default "0, 0, 0") (Hit :type Hit%20Result%20Structure%20%28by%20ref%29))
  ;[0 0 0] Arrow Collision
  (Game|Damage|ApplyDamage Other (Variables|Default|GetArrowDamage) (Game|GetInstigatorController) self)
  (CallFunction|MulticastEmitter)
  (Actor|SetLifeSpan 4.0))

(event EventBeginPlay
  ;[1 1 1] Setting Velocity to 0 in projectile movement then enabling this (fixes impact collision for client) See - https://forums.unrealengine.com/development-discussion/blueprint-visual-scripting/93551-multiplayer-fast-projectiles-issues
)

(fn ConstructionScript)