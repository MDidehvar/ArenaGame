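; Ultimate arrow projectile intended to home in on a target, applying damage on hit.
; HomingTest toggles a gated Tick that updates look-at rotation and re-aims velocity along the facing, scaling speed by 1.1 each tick.
; Overlapping the HomingTest target, unless it is player 0, spawns an explosion once and destroys the arrow.
; BeginPlay is empty; the launch velocity, lifespan and multicast effect calls are unwired.
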(event OnComponentBeginOverlap(SphereCollision)
  (params (OverlappedComponent :type Primitive%20Component%20Object%20Reference) (OtherActor :type Actor%20Object%20Reference) (OtherComp :type Primitive%20Component%20Object%20Reference) (OtherBodyIndex :type Integer) (bFromSweep :type Boolean) (SweepResult :type Hit%20Result%20Structure%20%28by%20ref%29))
  (if (not (== OtherActor (Game|GetPlayerCharacter 0)))
    (if (== OtherActor (stale Custom|HomingTest NewParam))
      (Utilities|FlowControl|DoOnce false
        (:Completed
          (Effects|SpawnEmitteratLocation "/Game/Extras/FX/P_Grenade_Explosion_01.P_Grenade_Explosion_01" (Transformation|GetActorLocation OtherActor))
          (Actor|DestroyActor))))))

(event Custom|HomingTest
  (params (NewParam :type Actor%20Object%20Reference))
  (bind _returnvalue (Transformation|GetActorRotation))
  ;[1 1 1] Makes projectile always turn toward target
  (Utilities|FlowControl|Gate true) ; enters at Toggle
)

(event Custom|MulticastEmitter
  ;[0 0 0] Arrow Collision
  (Effects|SpawnEmitteratLocation (Variables|Default|GetHitEffect) (Transformation|GetActorLocation)))

(event EventTick
  (params (DeltaSeconds :type Float%20%28single-precision%29))
  (bind _returnvalue (Transformation|GetActorRotation))
  ;[1 1 1] Makes projectile always turn toward target
  (Utilities|FlowControl|Gate true
    (:Exit
      (Transformation|SetActorRotation (Math|Rotator|FindLookatRotation (Transformation|GetActorLocation) (Transformation|GetActorLocation)))
      (Variables|/Script/Engine.MovementComponent|SetVelocity (Variables|Default|GetProjectileMovement) (* (Class|KismetMathLibrary|CreateVectorfromYawPitch (.yaw _returnvalue) (.pitch _returnvalue) (Math|Vector|VectorLength (Transformation|GetVelocity))) 1.1)))))

(event Collision|EventHit
  (params (MyComp :type Primitive%20Component%20Object%20Reference) (Other :type Actor%20Object%20Reference) (OtherComp :type Primitive%20Component%20Object%20Reference) (bSelfMoved :type Boolean) (HitLocation :type Vector :default "0, 0, 0") (HitNormal :type Vector :default "0, 0, 0") (NormalImpulse :type Vector :default "0, 0, 0") (Hit :type Hit%20Result%20Structure%20%28by%20ref%29))
  ;[0 0 0] Arrow Collision
  (Game|Damage|ApplyDamage Other (Variables|Default|GetArrowDamage) (Game|GetInstigatorController) self))

(event EventBeginPlay
  ;[1 1 1] Setting Velocity to 0 in projectile movement then enabling this (fixes impact collision for client) See - https://forums.unrealengine.com/development-discussion/blueprint-visual-scripting/93551-multiplayer-fast-projectiles-issues
)

(fn ConstructionScript)